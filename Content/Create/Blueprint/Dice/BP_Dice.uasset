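; BP_Dice is a die actor that tells the board when it comes to rest.
; When the Dice component goes to sleep, it finds BP_Board by class and calls EvtBoard without passing a value.
; Face detection by hit boxes is unfinished: only Box4 records a face enum.
; The rotation getter and the debug Switch, which prints each face's opposite value, are not called from live logic.
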(event `self.ReceiveTick`
  (params (DeltaSeconds :type "Float (single-precision)")))

(event `self.ReceiveBeginPlay`)

(event `self.ReceiveActorBeginOverlap`
  (params (OtherActor :type "Actor Object Reference")))

(event `self.Box4.OnComponentHit`
  (params (HitComponent :type "PrimitiveComponent Object Reference") (OtherActor :type "Actor Object Reference") (OtherComp :type "PrimitiveComponent Object Reference") (NormalImpulse :type "Vector Structure") (Hit :type "HitResult Structure (by ref)"))
  (if true
    (set `self.EN_Render` "NewEnumerator2")))

(event `self.Box5.OnComponentHit`
  (params (HitComponent :type "PrimitiveComponent Object Reference") (OtherActor :type "Actor Object Reference") (OtherComp :type "PrimitiveComponent Object Reference") (NormalImpulse :type "Vector Structure") (Hit :type "HitResult Structure (by ref)")))

(event `self.Dice.OnComponentSleep`
  (params (SleepingComponent :type "PrimitiveComponent Object Reference") (BoneName :type Name))
  (bind _returnvalue (`GameplayStatics.GetActorOfClass` "/Game/Create/Blueprint/Dice/BP_Board.BP_Board_C"))
  (`/Game/Create/Blueprint/Dice/BP_Board.Evt_Board` _returnvalue))

(fn `Dice_Roll`
  (returns (Output_Get :type "Rotator Structure"))
  (bind _output_get (set `self.Roll` (`SceneComponent.RelativeRotation` (`self.Dice`))))
  (return _output_get))

(fn `Switch`
  (params (RenderNum :type "/Game/Create/Blueprint/EN_RenderNumber Enum" :default "NewEnumerator0"))
  (switch `/Game/Create/Blueprint/EN_RenderNumber` RenderNum
    (:`NewEnumerator0`
      (`KismetSystemLibrary.PrintString` "NONE,NONE"))
    (:`NewEnumerator1`
      (`KismetSystemLibrary.PrintString` "6666"))
    (:`NewEnumerator2`
      (`KismetSystemLibrary.PrintString` "5555"))
    (:`NewEnumerator3`
      (`KismetSystemLibrary.PrintString` "4444"))
    (:`NewEnumerator4`
      (`KismetSystemLibrary.PrintString` "3333"))
    (:`NewEnumerator5`
      (`KismetSystemLibrary.PrintString` "2222"))
    (:`NewEnumerator6`
      (`KismetSystemLibrary.PrintString` "1111"))))

(fn `UserConstructionScript`)