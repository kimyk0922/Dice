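; BP_Board is a dice board that detects which side of a BP_Dice rests on it, apparently an unfinished prototype.
; Evt_Board finds the dice actor and tests its face boxes against the board's Box in a nested branch chain, printing a face value.
; The chain is incomplete, with placeholder values and unwired checks.
; BeginPlay and Roll are empty, and the roll-rotation debug graph never runs.
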(event `Evt_Board`
  (bind _box (`self.Box`))
  (bind _returnvalue (`GameplayStatics.GetActorOfClass` "/Game/Create/Blueprint/Dice/BP_Dice.BP_Dice_C"))
  (if (`PrimitiveComponent.IsOverlappingComponent` (`/Game/Create/Blueprint/Dice/BP_Dice.Box1` _returnvalue) _box)
    (`KismetSystemLibrary.PrintString` "6")
    (elif (`PrimitiveComponent.IsOverlappingComponent` (`/Game/Create/Blueprint/Dice/BP_Dice.Box6` _returnvalue) _box)
      (`KismetSystemLibrary.PrintString` "1")
      (elif (`PrimitiveComponent.IsOverlappingComponent` (`/Game/Create/Blueprint/Dice/BP_Dice.Box4` _returnvalue) null)
        (`KismetSystemLibrary.PrintString` "1")
        (elif (`PrimitiveComponent.IsOverlappingComponent` (`/Game/Create/Blueprint/Dice/BP_Dice.Box5` _returnvalue) _box)
          (`KismetSystemLibrary.PrintString` "1")
          (elif (`PrimitiveComponent.IsOverlappingComponent` (`/Game/Create/Blueprint/Dice/BP_Dice.Box3` _returnvalue) null)
            _))))))

(event `self.ReceiveBeginPlay`)

(fn `Roll`)

(fn `UserConstructionScript`)