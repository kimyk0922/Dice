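; BP_Gamble is a three-cup gambling prop, apparently a shell game, with left, center and right cups.
; BeginPlay places the outer cups at their Y offsets; Evt_Play runs Shuffle, then repositions all three and prints the offsets.
; Shuffle swaps and shuffles a temporary L/C/R array without assigning results back to those variables.
; Evt_LeftOpen tilts and lifts CupL in capped incremental steps, without delays, then resets the counter.
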(event `self.ReceiveBeginPlay`
  (`self.SetOffset`))

(event `Evt_Play`
  (`self.Shuffle`)
  (`self.Offset`))

(event `Evt_LeftOpen`
  (bind _output_get (set `self.Anim_Open` (`self.Anim_Open`)))
  (for _ (range 4)
    (`self.Open` (`self.Cup_L`)))
  (set `self.Anim_Open` 0))

(fn `Offset`
  (bind _l (`self.L`))
  (bind _c (`self.C`))
  (bind _r (`self.R`))
  (`SceneComponent.K2_SetRelativeLocation` (`self.Cup_L`) (`KismetMathLibrary.MakeVector` 0.0 _l) false false)
  (`SceneComponent.K2_SetRelativeLocation` (`self.Cup_R`) (`KismetMathLibrary.MakeVector` 0.0 _r) false false)
  (`SceneComponent.K2_SetRelativeLocation` (`self.Cup_C`) (`KismetMathLibrary.MakeVector` 0.0 _c) false false)
  (`KismetSystemLibrary.PrintString` (`KismetStringLibrary.Concat_StrStr` "L : " (`KismetStringLibrary.Conv_DoubleToString` _l) "/ C : " (`KismetStringLibrary.Conv_DoubleToString` _c) "/ R : " (`KismetStringLibrary.Conv_DoubleToString` _r)) true true (struct :`G` 0.66 :`B` 1.0 :`A` 1.0) 10.0))

(fn `Open`
  (params (Target :type "SceneComponent Object Reference"))
  (`KismetSystemLibrary.PrintString` "Left")
  (if (< (`self.Anim_Open`) 3)
    (`SceneComponent.K2_AddLocalTransform` Target (`KismetMathLibrary.MakeTransform` (0.0 5.0 5.0) (struct :`Roll` 10.0)) false false)
    (set `self.Anim_Open` (+ (`self.Anim_Open`) 1))))

(fn `SetOffset`
  (`SceneComponent.K2_SetRelativeLocation` (`self.Cup_L`) (`KismetMathLibrary.MakeVector` 0.0 (`self.L`)) false false)
  (set `self.L` (`self.L`))
  (`SceneComponent.K2_SetRelativeLocation` (`self.Cup_R`) (`KismetMathLibrary.MakeVector` 0.0 (`self.R`)) false false)
  (set `self.R` (`self.R`))
  (set `self.C` (`self.C`)))

(fn `Shuffle`
  (bind _array (`|MakeArray` (`self.L`) (`self.C`) (`self.R`)))
  (while (< (`self.Shuffle_Value`) 3)
    (`KismetArrayLibrary.Array_Swap` _array 0 (`KismetArrayLibrary.Array_Length` _array))
    (set `self.Shuffle_Value` (+ (`self.Shuffle_Value`) 1)))
  (`KismetArrayLibrary.Array_Shuffle` _array))

(fn `UserConstructionScript`)